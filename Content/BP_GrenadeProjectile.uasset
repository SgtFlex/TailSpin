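; Grenade projectile that goes off on a timed fuse, built on a parent projectile class.
; BeginPlay waits out a short delay, calls ProjectileHitEffects with the last stored overlap, then destroys the actor.
; The Sphere's begin-overlap event only records its sweep result as LastOverlap.
; The ProjectileOverlap override returns without reaching its parent call, so the parent's overlap response is suppressed.
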(event `self.ReceiveBeginPlay`
  (`parent.ReceiveBeginPlay`)
  (`KismetSystemLibrary.Delay` 2.0)
  (`self.ProjectileHitEffects` (`self.LastOverlap`))
  (`self.K2_DestroyActor`))

(event `self.Sphere.OnComponentBeginOverlap`
  (params (OverlappedComponent :type "PrimitiveComponent Object Reference") (OtherActor :type "Actor Object Reference") (OtherComp :type "PrimitiveComponent Object Reference") (OtherBodyIndex :type Integer) (bFromSweep :type Boolean) (SweepResult :type "HitResult Structure (by ref)"))
  (set `self.LastOverlap` SweepResult))

(fn `ProjectileOverlap`
  (params (DamagedActor :type "Actor Object Reference") (HitInfo :type "HitResult Structure (by ref)"))
  (return))

(fn `UserConstructionScript`
  (`parent.UserConstructionScript`))