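; Health component that tracks an owning actor's current health between zero and a maximum.
; AddHealth and SubtractHealth both route through ChangeHealth, which clamps the new value and broadcasts OnHealthChanged with instigator, causer and owner.
; OnHealthDepleted also fires on any change that leaves health at zero, including repeat hits, as no already-depleted guard exists.
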(fn `AddHealth`
  (params (AddedHealth :type "Float (double-precision)") (Instigator :type "Controller Object Reference") (Causer :type "Actor Object Reference"))
  (`self.ChangeHealth` (+ (`self.CurrentHealth`) AddedHealth) Instigator Causer))

(fn `ChangeHealth`
  (params (CurrentHealth :type "Float (double-precision)") (Instigator :type "Controller Object Reference") (Causer :type "Actor Object Reference"))
  (bind _returnvalue (`self.GetOwner`))
  (bind _output_get (set `self.CurrentHealth` (`KismetMathLibrary.FClamp` CurrentHealth 0.0 (`self.MaxHealth`))))
  (`self.OnHealthChanged` Instigator Causer _returnvalue)
  (if (<= _output_get 0.0)
    (`self.OnHealthDepleted` Causer Instigator _returnvalue)))

(fn `SubtractHealth`
  (params (SubtractedHealth :type "Float (double-precision)") (Instigator :type "Controller Object Reference") (Causer :type "Actor Object Reference"))
  (`self.ChangeHealth` (- (`self.CurrentHealth`) SubtractedHealth) Instigator Causer))