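; BP_ProjectileBase is a base projectile that deals point damage to the first actor its sphere overlaps, ignoring its owner.
; On overlap it spawns an impact particle system and sound, applies damage credited to the instigator's controller, then destroys itself.
; The particle system spawns at the projectile's location facing along the impact normal, while the sound plays at the impact point.
; The damage call passes the sweep location as its hit direction.
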(event `self.Sphere.OnComponentBeginOverlap`
  (params (OverlappedComponent :type "PrimitiveComponent Object Reference") (OtherActor :type "Actor Object Reference") (OtherComp :type "PrimitiveComponent Object Reference") (OtherBodyIndex :type Integer) (bFromSweep :type Boolean) (SweepResult :type "HitResult Structure (by ref)"))
  (if (!= OtherActor (`self.GetOwner`))
    (`self.ProjectileHitEffects` SweepResult)
    (`GameplayStatics.ApplyPointDamage` OtherActor (`self.Base Damage`) (`.Location` (`GameplayStatics.BreakHitResult` SweepResult)) SweepResult (`self.GetInstigatorController`) self "/Script/Engine.DamageType")
    (`self.K2_DestroyActor`)))

(fn `ProjectileHitEffects`
  (params (Hit :type "HitResult Structure"))
  (bind (_bblockinghit _binitialoverlap _time _distance _location _impactpoint _normal _impactnormal) (`GameplayStatics.BreakHitResult` Hit))
  (`NiagaraFunctionLibrary.SpawnSystemAtLocation` (`self.ProjectileHitPS`) (`self.K2_GetActorLocation`) (`KismetMathLibrary.Conv_VectorToRotator` _impactnormal))
  (`GameplayStatics.SpawnSoundAtLocation` (`self.HitSound`) _impactpoint (struct) 1.0 1.0 0.0 null null))

(fn `UserConstructionScript`)