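; Base weapon actor that fires projectiles along its forward vector, with sound and Niagara effects.
; StartFiring fires once immediately, then loops Fire on a timer until StopFiring clears it.
; The timer interval is FireRate divided by the instigator player controller's FireRateMultiplier, read only at start, so instigators without BP_PlayerController get just the single shot.
; Each shot spawns ProjectileClass just ahead of the weapon, passing on owner and instigator.
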(fn `Fire`
  (`self.SpawnProjectile`)
  (`GameplayStatics.SpawnSoundAttached` (`self.StartFireSound`) (`self.DefaultSceneRoot`) "None" (0.0 0.0 0.0) (struct) "KeepRelativeOffset" false 1.0 1.0 0.0 null null))

(fn `SpawnProjectile`
  (`|SpawnActorFromClass` (`self.ProjectileClass`) (`KismetMathLibrary.MakeTransform` (+ (`self.K2_GetActorLocation`) (* (`self.GetActorForwardVector`) 100.0)) (`self.K2_GetActorRotation`)) "AdjustIfPossibleButAlwaysSpawn" "MultiplyWithRoot" (`self.GetOwner`) (`self.GetInstigator`))
  (`self.SpawnProjectileEffects`))

(fn `SpawnProjectileEffects`
  (`GameplayStatics.SpawnSoundAttached` (`self.FireProjectileSound`) (`self.DefaultSceneRoot`) "None" (0.0 0.0 0.0) (struct) "KeepRelativeOffset" false 1.0 1.0 0.0 null null)
  (`NiagaraFunctionLibrary.SpawnSystemAttached` (`self.SpawnProjectilePS`) (`self.DefaultSceneRoot`) "None" (0.0 0.0 0.0) (struct) "KeepRelativeOffset" true))

(fn `StartFiring`
  (`self.Fire`)
  (bind _asbp_player_controller (cast `/Game/BP_PlayerController` (`Pawn.GetController` (`self.GetInstigator`))))
  (bind _returnvalue (`KismetSystemLibrary.K2_SetTimer` null "Fire" (/ (`self.FireRate`) (`/Game/BP_PlayerController.FireRateMultiplier` _asbp_player_controller)) true false 0.0 (`self.StartDelay`)))
  (set `self.FiringTimer` _returnvalue))

(fn `StopFiring`
  (`KismetSystemLibrary.K2_ClearAndInvalidateTimerHandle` (`self.FiringTimer`)))

(fn `UserConstructionScript`)