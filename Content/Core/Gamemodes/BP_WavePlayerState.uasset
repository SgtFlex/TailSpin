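; Player state for the wave game mode that tracks score and owns the main player-facing screens.
; On BeginPlay it creates the HUD widget for the player's helicopter character.
; All score edits route through ChangeScore, which fires ScoreChanged and opens a card selection screen whenever the score lands on a multiple of ten.
; It also provides a death screen function; IncreaseMaxHealth is an empty stub.
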(event `self.ReceiveBeginPlay`
  (bind _asbp_heli_character (cast `/Game/BP_HeliCharacter` (`GameplayStatics.GetPlayerCharacter` 0)))
  (bind _returnvalue (`|CreateWidget` "/Game/UI/WBP_PlayerHUD.WBP_PlayerHUD_C" null _asbp_heli_character))
  (bind _output_get (set `self.WaveHUD` _returnvalue))
  (`UserWidget.AddToPlayerScreen` _output_get 0))

(fn `AddGameOverScreen`
  (bind _returnvalue (`|CreateWidget` "/Game/UI/WBP_DeathScreen.WBP_DeathScreen_C" (`self.GetPlayerController`)))
  (`UserWidget.AddToPlayerScreen` _returnvalue 0))

(fn `AddScore`
  (params (AddScore :type "Float (double-precision)"))
  (`self.ChangeScore` (+ (`self.WaveScore`) AddScore)))

(fn `ChangeScore`
  (params (NewScore :type "Float (double-precision)"))
  (bind _output_get (set `self.WaveScore` NewScore))
  (`self.ScoreChanged` _output_get)
  (if (== (mod _output_get 10.0) 0.0)
    (bind _returnvalue (`|CreateWidget` "/Game/UI/WBP_CardSelectionScreen.WBP_CardSelectionScreen_C" (`GameplayStatics.GetPlayerController` 0)))
    (`UserWidget.AddToPlayerScreen` _returnvalue 0)))

(fn `IncreaseMaxHealth`)

(fn `SubtractScore`
  (params (SubScore :type "Float (double-precision)"))
  (`self.ChangeScore` (- (`self.WaveScore`) SubScore)))

(fn `UserConstructionScript`)