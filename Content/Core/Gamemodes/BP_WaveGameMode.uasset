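; BP_WaveGameMode is the game mode that continuously spawns enemies around the player and handles scoring and game over.
; A looping timer calls SpawnWave, which line-traces down from random points around the first player's pawn to spawn a random AI-controlled enemy.
; Health component depletion events are bound on enemies and helicopter pawns, with kill handlers updating BP_WavePlayerState.
; Tick scales Difficulty with real time, though nothing here reads it.
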(event `self.ReceiveBeginPlay`
  (`self.SpawnWave`)
  (`KismetSystemLibrary.K2_SetTimer` null "SpawnWave" 0.5 true))

(event `EnemyKilled`
  (params (Causer :type "Actor Object Reference") (Instigator :type "Controller Object Reference") (Owner :type "Actor Object Reference"))
  (bind _asplayer_controller (cast `PlayerController` Instigator))
  (bind _asbp_wave_player_state (cast `/Game/Core/Gamemodes/BP_WavePlayerState` (`Controller.PlayerState` _asplayer_controller)))
  (`/Game/Core/Gamemodes/BP_WavePlayerState.AddScore` _asbp_wave_player_state 1.0))

(event `PlayerKilled`
  (params (Causer :type "Actor Object Reference") (Instigator :type "Controller Object Reference") (Owner :type "Actor Object Reference"))
  (bind _asbp_heli_character (cast `/Game/BP_HeliCharacter` Owner))
  (bind _asbp_wave_player_state (cast `/Game/Core/Gamemodes/BP_WavePlayerState` (`Pawn.PlayerState` _asbp_heli_character)))
  (`/Game/Core/Gamemodes/BP_WavePlayerState.AddGameOverScreen` _asbp_wave_player_state))

(event `self.ReceiveTick`
  (params (DeltaSeconds :type "Float (single-precision)"))
  (set `self.Difficulty` (/ (`GameplayStatics.GetRealTimeSeconds`) 10.0)))

(fn `SpawnDefaultPawnFor`
  (params (NewPlayer :type "Controller Object Reference") (StartSpot :type "Actor Object Reference"))
  (returns (ReturnValue :type "Pawn Object Reference"))
  (bind _returnvalue (`parent.SpawnDefaultPawnFor` NewPlayer StartSpot))
  (bind _asbp_heli_character (cast `/Game/BP_HeliCharacter` _returnvalue))
  (add `/Game/Core/Components/BP_HealthComponent.OnHealthDepleted` (`/Game/BP_HeliCharacter.BP_HealthComponent` _asbp_heli_character) (`|CreateDelegate` :!event `PlayerKilled`))
  (return _returnvalue))

(fn `SpawnWave`
  (bind (_returnvalue_x _returnvalue_y) (`KismetMathLibrary.BreakVector` (`KismetMathLibrary.RandomUnitVector`)))
  (bind _returnvalue (+ (`self.K2_GetActorLocation` (`Controller.K2_GetPawn` (`GameplayStatics.GetPlayerController` 0))) (* (`KismetMathLibrary.Normal` (`KismetMathLibrary.MakeVector` _returnvalue_x _returnvalue_y)) (`KismetMathLibrary.RandomFloatInRange` 2000.0 2500.0))))
  (for _ (range 1)
    (bind _outhit (`KismetSystemLibrary.LineTraceSingle` :`Start` _returnvalue :`End` (+ _returnvalue (0.0 0.0 -5000.0)) :`TraceChannel` "TraceTypeQuery1" :`DrawDebugType` "ForDuration"))
    (bind _returnvalue_2 (`|SpawnActorFromClass` (`KismetArrayLibrary.Array_Random` (`self.Enemies`)) (`KismetMathLibrary.MakeTransform` (`.Location` (`GameplayStatics.BreakHitResult` _outhit))) "AdjustIfPossibleButAlwaysSpawn" "MultiplyWithRoot" null null))
    (`Pawn.SpawnDefaultController` _returnvalue_2)
    (add `/Game/Core/Components/BP_HealthComponent.OnHealthDepleted` (`/Game/Characters/Tank/BP_EnemyBase.BP_HealthComponent` _returnvalue_2) (`|CreateDelegate` :!event `EnemyKilled`))))

(fn `UserConstructionScript`)