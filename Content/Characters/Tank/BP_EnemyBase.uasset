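; BP_EnemyBase is a base enemy that takes damage, dies, and fires a child-actor weapon.
; On BeginPlay it multiplies its health component's current health by the wave game mode's Difficulty and sets max health to match.
; AnyDamage subtracts health through that component, whose depletion event destroys the actor.
; A Fire event forwards to the child BP_WeaponBase, while a StartFiring call is left unconnected.
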(event `Fire`
  (bind _asbp_weapon_base (cast `/Game/Core/BP_WeaponBase` (`ChildActorComponent.ChildActor` (`self.ChildActor`))))
  (`/Game/Core/BP_WeaponBase.Fire` _asbp_weapon_base))

(event `self.ReceiveBeginPlay`
  (bind _bp_healthcomponent (`self.BP_HealthComponent`))
  (bind _asbp_wave_game_mode (cast `/Game/Core/Gamemodes/BP_WaveGameMode` (`GameplayStatics.GetGameMode`)))
  (bind _output_get (set `/Game/Core/Components/BP_HealthComponent.CurrentHealth` (* (`/Game/Core/Components/BP_HealthComponent.CurrentHealth` _bp_healthcomponent) (`/Game/Core/Gamemodes/BP_WaveGameMode.Difficulty` _asbp_wave_game_mode)) _bp_healthcomponent))
  (set `/Game/Core/Components/BP_HealthComponent.MaxHealth` _output_get _bp_healthcomponent))

(event `self.BP_HealthComponent.OnHealthDepleted`
  (params (Causer :type "Actor Object Reference") (Instigator :type "Controller Object Reference") (Owner :type "Actor Object Reference"))
  (`self.K2_DestroyActor`))

(event `self.ReceiveAnyDamage`
  (params (Damage :type "Float (single-precision)") (DamageType :type "DamageType Object Reference") (InstigatedBy :type "Controller Object Reference") (DamageCauser :type "Actor Object Reference"))
  (`/Game/Core/Components/BP_HealthComponent.SubtractHealth` (`self.BP_HealthComponent`) Damage InstigatedBy DamageCauser))

(fn `UserConstructionScript`)