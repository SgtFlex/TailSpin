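; Flare countermeasure weapon that launches flares to draw homing projectiles away from its owning character.
; Firing starts on BeginPlay and again whenever ammo finishes regenerating.
; Each shot spawns four flares at even yaw intervals, then retargets each incoming homing projectile onto a random entry in the fired flares list and makes the owning character its instigator.
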(event `self.ReceiveBeginPlay`
  (`parent.ReceiveBeginPlay`)
  (`self.StartFiring`)
  (add `self.OnAmmoFinishedRegenerating` (delegate `FireWhenFull`)))

(event `FireWhenFull`
  (`self.StartFiring`))

(fn `Fire`
  (locals (FiredFlares :type "Array of /Game/Core/BP_ProjectileBase Object Reference"))
  (`parent.Fire`))

(fn `SpawnProjectile`
  (locals (FiredFlares :type "Array of /Game/Core/BP_ProjectileBase Object Reference"))
  (for _index (range 4)
    (bind _returnvalue (`|SpawnActorFromClass` (`self.ProjectileClass`) (`KismetMathLibrary.MakeTransform` (`self.K2_GetActorLocation`) (`KismetMathLibrary.MakeRotator` 0.0 0.0 (* (/ 360.0 4.0) _index))) "AdjustIfPossibleButAlwaysSpawn" "MultiplyWithRoot" (`self.GetOwner`) (`self.GetInstigator`)))
    (`KismetArrayLibrary.Array_Add` (`local.FiredFlares`) _returnvalue))
  (for _array_element (`/Game/BP_HeliCharacter.IncomingHomingProjectiles` (`self.OwningCharacter`))
    (`/Engine/EditorBlueprintResources/StandardMacros.IsValid` _array_element
      (:`Is Valid`
        (set `ProjectileMovementComponent.HomingTargetComponent` (`Actor.RootComponent` (`KismetArrayLibrary.Array_Random` (`local.FiredFlares`))) (`/Game/Core/BP_ProjectileBase.ProjectileMovement` _array_element))
        (set `Actor.Instigator` (`self.OwningCharacter`) _array_element)))))

(fn `UserConstructionScript`
  (`parent.UserConstructionScript`))