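; Player controller that caches the possessed BP_HeliCharacter and provides stat upgrade functions, each scaling by a compounding 10% factor.
; Health, regen, spin, speed and handling upgrades write straight to the helicopter, its health component or movement component.
; Weapon damage, fire rate and ammo upgrades only adjust multipliers stored on the controller.
; IncreaseAmmoRegenSpeed changes the same delay multiplier as DecreaseAmmoRegenDelay, with no separate speed value.
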(event `self.ReceivePossess`
  (params (PossessedPawn :type "Pawn Object Reference"))
  (bind _asbp_heli_character (cast `/Game/BP_HeliCharacter` PossessedPawn))
  (set `self.As BP Heli Character` _asbp_heli_character)
  (`parent.ReceivePossess` PossessedPawn))

(fn `DecreaseAmmoRegenDelay`
  (set `self.AmmoRegenDelayMultiplier` (/ (`self.AmmoRegenDelayMultiplier`) 1.1)))

(fn `DecreaseHealthRegenDelay`
  (bind _as_bp_heli_character (`self.As BP Heli Character`))
  (set `/Game/BP_HeliCharacter.HealthRegenDelay` (/ (`/Game/BP_HeliCharacter.HealthRegenDelay` _as_bp_heli_character) 1.1) _as_bp_heli_character))

(fn `IncreaseAmmoRegenSpeed`
  (set `self.AmmoRegenDelayMultiplier` (/ (`self.AmmoRegenDelayMultiplier`) 1.1)))

(fn `IncreaseControl`
  (bind _charactermovement (`Character.CharacterMovement` (`self.As BP Heli Character`)))
  (set `CharacterMovementComponent.MaxAcceleration` (* (`CharacterMovementComponent.MaxAcceleration` _charactermovement) 1.1) _charactermovement)
  (set `CharacterMovementComponent.BrakingDecelerationFlying` (* (`CharacterMovementComponent.BrakingDecelerationFlying` _charactermovement) 1.1) _charactermovement))

(fn `IncreaseFireRate`
  (set `self.FireRateMultiplier` (* (`self.FireRateMultiplier`) 1.1)))

(fn `IncreaseHealthRegenSpeed`
  (bind _as_bp_heli_character (`self.As BP Heli Character`))
  (set `/Game/BP_HeliCharacter.HealthRegenAmount` (* (`/Game/BP_HeliCharacter.HealthRegenAmount` _as_bp_heli_character) 1.1) _as_bp_heli_character))

(fn `IncreaseMaxAmmo`
  (set `self.AmmoMaxMultiplier` (* (`self.AmmoMaxMultiplier`) 1.1)))

(fn `IncreaseMaxHealth`
  (bind _bp_healthcomponent (`/Game/BP_HeliCharacter.BP_HealthComponent` (`self.As BP Heli Character`)))
  (set `/Game/Core/Components/BP_HealthComponent.MaxHealth` (* (`/Game/Core/Components/BP_HealthComponent.MaxHealth` _bp_healthcomponent) 1.1) _bp_healthcomponent))

(fn `IncreaseMoveSpeed`
  (bind _charactermovement (`Character.CharacterMovement` (`self.As BP Heli Character`)))
  (set `CharacterMovementComponent.MaxFlySpeed` (* (`CharacterMovementComponent.MaxFlySpeed` _charactermovement) 1.1) _charactermovement))

(fn `IncreaseSpinSpeed`
  (set `/Game/BP_HeliCharacter.SpinRate` (* (`/Game/BP_HeliCharacter.SpinRate` (`self.As BP Heli Character`)) 1.1) (`self.As BP Heli Character`)))

(fn `IncreaseWeaponDamage`
  (set `self.DamageMultiplier` (* (`self.DamageMultiplier`) 1.1)))

(fn `UserConstructionScript`)