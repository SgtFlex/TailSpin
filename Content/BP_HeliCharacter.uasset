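; Player helicopter character with Enhanced Input movement, weapons and regenerating health.
; Tick yaws the mesh by SpinRate, eases TiltPivot toward the movement direction and sets a Niagara laser's end to the trace end, not the hit point.
; Weapons spawn attached to the mesh, starting with a gatling gun, and the selected one fires on input.
; Damage feeds BPHealthComponent and restarts timer-based regen; depletion explodes, hides and disables the heli.
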(event `self.ReceiveRestarted`
  (bind _asplayer_controller (cast `PlayerController` (`self.GetController`)))
  (`EnhancedInputSubsystemInterface.AddMappingContext` (pcsubsystem `EnhancedInputLocalPlayerSubsystem` _asplayer_controller) "/Game/Core/Inputs/IMC_Heli.IMC_Heli" 0 (struct)))

(event `self.ReceiveTick`
  (params (DeltaSeconds :type "Float (single-precision)"))
  (bind _tiltpivot (`self.TiltPivot`))
  (bind (_returnvalue_x _returnvalue_y) (`KismetMathLibrary.BreakVector` (* (`KismetMathLibrary.Normal` (`MovementComponent.Velocity` (`self.CharacterMovement`))) -10.0)))
  (`self.LaserTrace`)
  (`SceneComponent.K2_AddRelativeRotation` (`self.SkeletalMesh`) (`KismetMathLibrary.MakeRotator` 0.0 0.0 (* DeltaSeconds (`self.SpinRate`))) false false)
  (`SceneComponent.K2_SetRelativeRotation` _tiltpivot (`KismetMathLibrary.RLerp` (`SceneComponent.RelativeRotation` _tiltpivot) (`KismetMathLibrary.MakeRotator` _returnvalue_y (* _returnvalue_x -1.0)) (* DeltaSeconds 10.0)) false false))

(event `EnhancedInput|/Game/Core/Inputs/IA_MoveX`
  (params (ActionValue :type "Float (double-precision)") (ElapsedSeconds :type "Float (double-precision)") (TriggeredSeconds :type "Float (double-precision)") (InputAction :type "InputAction Object Reference" :default "/Game/Core/Inputs/IA_MoveX.IA_MoveX"))
  (:`Triggered`
    (`PawnMovementComponent.AddInputVector` (`self.CharacterMovement`) (`KismetMathLibrary.MakeVector` (* ActionValue 1000.0)) false)))

(event `EnhancedInput|/Game/Core/Inputs/IA_MoveY`
  (params (ActionValue :type "Float (double-precision)") (ElapsedSeconds :type "Float (double-precision)") (TriggeredSeconds :type "Float (double-precision)") (InputAction :type "InputAction Object Reference" :default "/Game/Core/Inputs/IA_MoveY.IA_MoveY"))
  (:`Triggered`
    (`PawnMovementComponent.AddInputVector` (`self.CharacterMovement`) (`KismetMathLibrary.MakeVector` 0.0 (* ActionValue 1000.0)) false)))

(event `EnhancedInput|/Game/Core/Inputs/IA_ShootPrimary`
  (params (ActionValue :type Boolean) (ElapsedSeconds :type "Float (double-precision)") (TriggeredSeconds :type "Float (double-precision)") (InputAction :type "InputAction Object Reference" :default "/Game/Core/Inputs/IA_ShootPrimary.IA_ShootPrimary"))
  (bind _selectedweapon (`self.SelectedWeapon`))
  (:`Started`
    (`/Game/Core/BP_WeaponBase.StartFiring` _selectedweapon))
  (:`Completed`
    (`/Game/Core/BP_WeaponBase.StopFiring` _selectedweapon)))

(event `self.ReceiveBeginPlay`
  (`parent.ReceiveBeginPlay`)
  (`self.AddWeapon` "/Game/Weapons/GatlingGun/BP_GatlingGun.BP_GatlingGun_C")
  (`self.SwitchToWeapon` 0))

(event `self.ReceiveAnyDamage`
  (params (Damage :type "Float (single-precision)") (DamageType :type "DamageType Object Reference") (InstigatedBy :type "Controller Object Reference") (DamageCauser :type "Actor Object Reference"))
  (`/Game/Core/Components/BP_HealthComponent.SubtractHealth` (`self.BP_HealthComponent`) Damage InstigatedBy DamageCauser)
  (`self.StopHealthRegen`)
  (`self.StartHealthRegenTimer`))

(event `self.BP_HealthComponent.OnHealthDepleted`
  (params (Causer :type "Actor Object Reference") (Instigator :type "Controller Object Reference") (Owner :type "Actor Object Reference"))
  (`SceneComponent.SetVisibility` (`self.SkeletalMesh`) false true)
  (`NiagaraFunctionLibrary.SpawnSystemAtLocation` "/Game/Sounds/NS_Explosion.NS_Explosion" (`self.K2_GetActorLocation`))
  (`self.DisableInput` null)
  (`MovementComponent.StopMovementImmediately` (`self.CharacterMovement`))
  (`self.SetActorEnableCollision` false))

(event `StartHealthRegeneration`
  (bind _returnvalue (`KismetSystemLibrary.K2_SetTimerDelegate` (delegate `RegenHealth`) 0.01 true))
  (set `self.HealthRegenTimerHandle` _returnvalue))

(event `RegenHealth`
  (bind _bp_healthcomponent (`self.BP_HealthComponent`))
  (`/Game/Core/Components/BP_HealthComponent.AddHealth` _bp_healthcomponent (`self.HealthRegenAmount`) null null)
  (if (>= (`/Game/Core/Components/BP_HealthComponent.CurrentHealth` _bp_healthcomponent) (`/Game/Core/Components/BP_HealthComponent.MaxHealth` _bp_healthcomponent))
    (`self.StopHealthRegen`)))

(event `StopHealthRegen`
  (`KismetSystemLibrary.K2_ClearAndInvalidateTimerHandle` (`self.HealthRegenTimerHandle`)))

(event `StartHealthRegenTimer`
  (bind _returnvalue (`KismetSystemLibrary.K2_SetTimerDelegate` (`|CreateDelegate` :!event `StartHealthRegeneration`) (`self.HealthRegenDelay`)))
  (set `self.HealthRegenDelayTimerHandle` _returnvalue))

(fn `AddWeapon`
  (params (AddedWeapon :type "/Game/Core/BP_WeaponBase Class Reference"))
  (returns (Weapon :type "/Game/Core/BP_WeaponBase Object Reference"))
  (bind _returnvalue (`|SpawnActorFromClass` AddedWeapon (`KismetMathLibrary.MakeTransform` (0.0 0.0 0.0)) "AlwaysSpawn" "MultiplyWithRoot" self self))
  (`self.K2_AttachToComponent` _returnvalue (`self.SkeletalMesh`) "None" "SnapToTarget" "SnapToTarget" "KeepRelative" true)
  (`self.K2_AddActorLocalRotation` _returnvalue (`KismetMathLibrary.MakeRotator` 0.0 0.0 90.0) false false)
  (`KismetArrayLibrary.Array_Add` (`self.WeaponCollection`) _returnvalue)
  (`self.WeaponAdded` _returnvalue)
  (return _returnvalue))

(fn `LaserTrace`
  (bind _skeletalmesh (`self.SkeletalMesh`))
  (bind _returnvalue (`SceneComponent.K2_GetComponentLocation` _skeletalmesh))
  (bind _outhit (`KismetSystemLibrary.LineTraceSingle` _returnvalue (+ _returnvalue (* (`SceneComponent.GetRightVector` _skeletalmesh) 3000.0) (0.0 0.0 -500.0)) "TraceTypeQuery1"))
  (`NiagaraComponent.SetVariableVec3` (`self.Niagara1`) "Beam End" (`.TraceEnd` (`GameplayStatics.BreakHitResult` _outhit))))

(fn `SwitchToWeapon`
  (params (Index :type Integer))
  (set `self.SelectedWeapon` (`|GetArrayItem` (`self.WeaponCollection`) Index)))

(fn `UserConstructionScript`
  (`parent.UserConstructionScript`))